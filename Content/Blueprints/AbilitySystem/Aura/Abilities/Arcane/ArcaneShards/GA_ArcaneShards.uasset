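; Arcane Shards gameplay ability that spawns a timed series of shard effects around a point targeted with the mouse.
; On activation it shows a magic circle, then waits for an input press to read the hit under the cursor.
; A spawned BP_PointCollection supplies ground points at random yaw, cached once.
; A looping timer fires the ArcaneShards gameplay cue at each point, then destroys the collection and ends the ability.
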(event `self.K2_ActivateAbility`
  (`|ExecutionSequence`
    (:`then_0`
      (message `PlayerInterface.ShowMagicCircle` (`self.GetAvatarActorFromActorInfo`) null))
    (:`then_1`
      (`AbilityTask_WaitInputPress.WaitInputPress` false
        (:`OnPress`
          (bind (_asynctaskproxy _datahandle) (`TargetDataUnderMouse.CreateTargetDataUnderMouse`)
            (:`ValidData`
              (bind (_bblockinghit _binitialoverlap _time _distance _location _impactpoint) (`GameplayStatics.BreakHitResult` (`AbilitySystemBlueprintLibrary.GetHitResultFromTargetData` _datahandle)))
              (if _bblockinghit
                (bind _returnvalue (`|SpawnActorFromClass` "/Game/Blueprints/AbilitySystem/Aura/Abilities/Arcane/ArcaneShards/BP_PointCollection.BP_PointCollection_C" (`KismetMathLibrary.MakeTransform` _impactpoint) "AlwaysSpawn" "MultiplyWithRoot" null null))
                (set `self.PointCollection` _returnvalue)
                ;[0 0 0 0.5] It's necessary to chache the array so it's not regenerated with each for loop iteration. Alternativly, we can simply use a non-pure function to get the array (keeping it pure only for educational purposes)
                (set `self.GroundPoints` (`PointCollection.GetGroundPoints` _returnvalue _impactpoint (`self.NumPoints`) (`KismetMathLibrary.RandomFloatInRange` 0.0 360.0)))
                (bind _returnvalue_2 (`KismetSystemLibrary.K2_SetTimerDelegate` (delegate `SpawnShard`) (`self.ShardSpawnDeltaTime`) true))
                (set `self.ShardSpawnTimer` _returnvalue_2)
                (`self.SpawnShard`)
                (message `PlayerInterface.HideMagicCircle` (`self.GetAvatarActorFromActorInfo`))
                (else
                  (`self.K2_EndAbility`))))))))))

(event `SpawnShard`
  (bind _returnvalue_location (`KismetMathLibrary.BreakTransform` (`SceneComponent.K2_GetComponentToWorld` (`|GetArrayItem` (`self.GroundPoints`) (`self.Count`)))))
  (if (< (`self.Count`) (`self.NumPoints`))
    (bind _output_get (set `self.ShardSpawnLocation` _returnvalue_location))
    (`/Engine/EditorBlueprintResources/StandardMacros.IncrementInt` (`self.Count`)
      (:`  `
        (`self.K2_ExecuteGameplayCueWithParams` (struct :`TagName` "GameplayCue.ArcaneShards") (`AbilitySystemBlueprintLibrary.MakeGameplayCueParameters` 0.0 0.0 (struct) (struct) (struct) (struct) (struct) (`self.ShardSpawnLocation`)))))
    (else
      (`KismetSystemLibrary.K2_ClearAndInvalidateTimerHandle` (`self.ShardSpawnTimer`))
      (`KismetSystemLibrary.Delay` 0.2)
      (`Actor.K2_DestroyActor` (`self.PointCollection`))
      (`self.K2_EndAbility`))))

(event `EndAbilityWithDelay`)

(event `self.K2_OnEndAbility`
  (params (bWasCancelled :type Boolean)))