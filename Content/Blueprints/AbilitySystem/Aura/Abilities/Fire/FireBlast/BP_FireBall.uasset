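; Fire Blast ability fireball that flies outward, then boomerangs back to ReturnToActor and explodes.
; On authority, one timeline lerps it to an apex ahead, then the ignore list is cleared and a second tracks ReturnToActor's live location.
; Within ExplodeDistance it calls OnHit, applies radial damage effects to nearby live players except itself and its owner, and destroys itself.
; Knockback pitch is overridden to launch victims upward; death impulse points away from the blast.
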(event `self.StartOutgoingTimeline`
  (`/Engine/EditorBlueprintResources/ActorMacros.Switch Has Authority`
    (:`Authority`
      ;[0.1451 0.15 0 0.5] Store Inital and Apex Locations
      (set `self.InitialLocation` (`self.K2_GetActorLocation`))
      (set `self.ApexLocation` (+ (`self.InitialLocation`) (* (`self.GetActorForwardVector`) (`self.TravelDistance`))))
      (bind (_direction _outgoingtrack) (`Timeline|OutgoingTimeline`)
        (:`Update`
          (`self.K2_SetActorLocation` (`KismetMathLibrary.VLerp` (`self.InitialLocation`) (`self.ApexLocation`) _outgoingtrack)))
        (:`Finished`
          (`self.EmptyIgnoreList`)
          (bind (_direction_2 _returningtrack) (`Timeline|RetruningTimeline`)
            (:`Update`
              (`self.K2_SetActorLocation` (`KismetMathLibrary.VLerp` (`self.ApexLocation`) (`self.K2_GetActorLocation` (`self.ReturnToActor`)) _returningtrack))
              (if (`self.IsWithinExplodDistance`)
                (`self.OnHit`)
                (bind _outoverlappingactors (`AuraAbilitySystemLibrary.GetLivePlayersWithinRadius` self (`|MakeArray` (`self.GetOwner`) self :!type "Actor Object Reference") (`self.RadialDamageOuterRadius`) (`self.K2_GetActorLocation`)))
                (set `self.OverlappingActors` _outoverlappingactors)
                (`AuraAbilitySystemLibrary.SetIsRadialDamageEffectParam` (`self.ExplosionDamageParams`) true (`self.RadialDamageInnerRadius`) (`self.RadialDamageOuterRadius`) (`self.K2_GetActorLocation`))
                (for _array_element (`self.OverlappingActors`)
                  (`AuraAbilitySystemLibrary.SetTargetEffectParamsASC` (`self.ExplosionDamageParams`) (`AbilitySystemBlueprintLibrary.GetAbilitySystemComponent` _array_element))
                  (set `self.KnockbackDirection` (- (`self.K2_GetActorLocation` _array_element) (`self.K2_GetActorLocation`)))
                  (`AuraAbilitySystemLibrary.SetKnockbackDirection` (`self.ExplosionDamageParams`) (`self.OverrideKnockbackPitch`) (`self.KnockbackMagnitude`))
                  (`AuraAbilitySystemLibrary.SetDeathImpulseDirection` (`self.ExplosionDamageParams`) (`self.KnockbackDirection`) (`self.DeathImpulseMagnitude`))
                  (`AuraAbilitySystemLibrary.ApplyDamageEffect` (`self.ExplosionDamageParams`)))
                (`self.K2_DestroyActor`)))))))))

(fn `IsWithinExplodDistance`
  (returns (ReturnValue :type Boolean))
  (return (<= (`KismetMathLibrary.VSize` (- (`self.K2_GetActorLocation`) (`self.K2_GetActorLocation` (`self.ReturnToActor`)))) (`self.ExplodeDistance`))))

(fn `OverrideKnockbackPitch`
  (returns (ReturnValue :type "Vector Structure"))
  (bind (_returnvalue_roll _returnvalue_pitch _returnvalue_yaw) (`KismetMathLibrary.BreakRotator` (`KismetMathLibrary.MakeRotFromX` (`self.KnockbackDirection`))))
  (return (`KismetMathLibrary.GetForwardVector` (`KismetMathLibrary.MakeRotator` _returnvalue_roll 45.0 _returnvalue_yaw))))

(fn `UserConstructionScript`)