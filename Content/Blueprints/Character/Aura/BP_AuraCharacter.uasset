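; Player character Blueprint for Aura, handling motion warping, shock loop state and fading of objects that overlap its box.
; UpdateFacingTarget feeds a location to the FacingTarget warp target, and SetinShockLoop stores a flag meant to be replicated for correct cues on client and server.
; Box overlaps send fade out/in messages through BI_FadeInterface, only when locally controlled and moving.
; Holding Tab halves global time dilation.
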(event `Key|Tab`
  (params (Key :type "Key Structure"))
  (:`Pressed`
    (`GameplayStatics.SetGlobalTimeDilation` 0.5))
  (:`Released`
    (`GameplayStatics.SetGlobalTimeDilation` 1.0)))

(event `CombatInterface.UpdateFacingTarget`
  (params (Target :type "Vector Structure (by ref)"))
  (`MotionWarpingComponent.AddOrUpdateWarpTargetFromLocation` (`self.MotionWarping`) "FacingTarget" Target))

(event `CombatInterface.SetInShockLoop`
  (params (bInLoop :type Boolean))
  ; Need to be replecated so the Cue is correct on client and server
  (set `self.InShockLoop` bInLoop))

(event `self.Box.OnComponentBeginOverlap`
  (params (OverlappedComponent :type "PrimitiveComponent Object Reference") (OtherActor :type "Actor Object Reference") (OtherComp :type "PrimitiveComponent Object Reference") (OtherBodyIndex :type Integer) (bFromSweep :type Boolean) (SweepResult :type "HitResult Structure (by ref)"))
  (if (`self.IsLocallyControlled`)
    (bind _moving (`self.IsMoving`))
    (if _moving
      (if (`KismetSystemLibrary.DoesImplementInterface` OtherActor "/Game/Blueprints/Actor/FadeActor/BI_FadeInterface.BI_FadeInterface_C")
        (message `/Game/Blueprints/Actor/FadeActor/BI_FadeInterface.FadeOut` OtherActor)))))

(event `self.Box.OnComponentEndOverlap`
  (params (OverlappedComponent :type "PrimitiveComponent Object Reference") (OtherActor :type "Actor Object Reference") (OtherComp :type "PrimitiveComponent Object Reference") (OtherBodyIndex :type Integer))
  (if (`self.IsLocallyControlled`)
    (bind _moving (`self.IsMoving`))
    (if _moving
      (if (`KismetSystemLibrary.DoesImplementInterface` OtherActor "/Game/Blueprints/Actor/FadeActor/BI_FadeInterface.BI_FadeInterface_C")
        (message `/Game/Blueprints/Actor/FadeActor/BI_FadeInterface.FadeIn` OtherActor)))))

(fn `IsMoving`
  (returns (Moving :type Boolean))
  (return (> (`KismetMathLibrary.VSize` (`MovementComponent.Velocity` (`self.CharacterMovement`))) 0.0)))

(fn `UserConstructionScript`)