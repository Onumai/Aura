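; BP_TestFindPathToLocation is a debug test actor that visualizes how query extents affect navmesh pathfinding from the world origin to its location.
; Every Tick it draws default and custom extent boxes, then pathfinds synchronously to both the raw location and that location projected with the custom extent.
; A shared event draws each path's points as differently colored spheres, showing that pathfinding still uses the default extent, while projection can search wider.
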(event `self.ReceiveTick`
  (params (DeltaSeconds :type "Float (single-precision)"))
  (bind (_projectedlocation _returnvalue) (`NavigationSystemV1.K2_ProjectPointToNavigation` (`self.K2_GetActorLocation`) null null (`self.CustomQueryContext`)))
  (`|ExecutionSequence`
    (:`then_0`
      ;[0.01096 0.01161 0.0137] Get path to the actor location, which uses the Default Query Extent to find points.
      (`KismetSystemLibrary.DrawDebugBox` (`self.K2_GetActorLocation`) (`self.Default QueryContext`) (struct :`B` 1.0 :`A` 1.0))
      (`self.FindPathToLocation` (`self.K2_GetActorLocation`) 10.0 (struct :`G` 1.0 :`B` 1.0 :`A` 1.0)))
    (:`then_1`
      ;[0.01096 0.01161 0.0137] Get path to the actor location projected to the NavMesh, using a custom (larger than default) Query Extent to find the projected point. NOTE: FindPathToLocation still uses the Default Query Context.
      (`KismetSystemLibrary.DrawDebugBox` (`self.K2_GetActorLocation`) (`self.CustomQueryContext`) (struct :`G` 1.0 :`A` 1.0))
      (if _returnvalue
        (`KismetSystemLibrary.DrawDebugSphere` _projectedlocation 30.0 12 (struct :`R` 1.0 :`A` 1.0))
        (`self.FindPathToLocation` _projectedlocation 20.0 (struct :`R` 1.0 :`G` 1.0 :`A` 1.0))))))

(event `FindPathToLocation`
  (params (Location :type "Vector Structure") (SphereRadius :type "Float (double-precision)") (DebugColor :type "LinearColor Structure"))
  (bind _returnvalue (`NavigationSystemV1.FindPathToLocationSynchronously` (`KismetMathLibrary.Vector_Zero`) Location null null))
  (`/Engine/EditorBlueprintResources/StandardMacros.IsValid` _returnvalue
    (:`Is Valid`
      (bind _pathpoints (`NavigationPath.PathPoints` _returnvalue))
      (if (> (`KismetArrayLibrary.Array_Length` _pathpoints) 0)
        (for _array_element _pathpoints
          (`KismetSystemLibrary.DrawDebugSphere` _array_element SphereRadius 12 DebugColor))))))

(fn `UserConstructionScript`)